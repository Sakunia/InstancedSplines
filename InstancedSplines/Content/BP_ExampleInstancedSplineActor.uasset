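; Example actor that tiles a static mesh along a spline using an instanced spline mesh component.
; The construction script clears and rebuilds the instances, deriving the segment count from spline length and the mesh's X bounds, rounded up.
; Segments are evenly resized to cover the whole spline exactly.
; Each instance takes its endpoints and tangents from the spline, with tangents normalized and scaled to segment length for smooth deformation.
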(fn `UserConstructionScript`
  (locals (MeshLength :type "Float (double-precision)" :default 200.0))
  (bind _spline (`self.Spline`))
  (bind _instancedsplinemesh (`self.InstancedSplineMesh`))
  (bind _returnvalue (`SplineComponent.GetSplineLength` (`self.Spline`)))
  (bind (_returnvalue_origin _returnvalue_boxextent) (`KismetMathLibrary.BreakBoxSphereBounds` (`StaticMesh.GetBounds` (`StaticMeshComponent.StaticMesh` _instancedsplinemesh))))
  (bind _returnvalue_2 (`KismetMathLibrary.FCeil` (/ _returnvalue (* (.x _returnvalue_boxextent) 2.0))))
  (`InstancedStaticMeshComponent.ClearInstances` _instancedsplinemesh)
  (set `local.MeshLength` (/ _returnvalue (`KismetMathLibrary.Conv_IntToDouble` _returnvalue_2)))
  (for _index (range _returnvalue_2)
    (bind _returnvalue_3 (* _index (`local.MeshLength`)))
    (bind _returnvalue_4 (* (+ _index 1) (`local.MeshLength`)))
    (`InstancedSplineMeshComponent.AddSplineInstance` (`self.InstancedSplineMesh`) (`SplineComponent.GetLocationAtDistanceAlongSpline` _spline _returnvalue_3 "Local") (* (`KismetMathLibrary.Normal` (`SplineComponent.GetTangentAtDistanceAlongSpline` _spline _returnvalue_3 "Local")) (`local.MeshLength`)) (`SplineComponent.GetLocationAtDistanceAlongSpline` _spline _returnvalue_4 "Local") (* (`KismetMathLibrary.Normal` (`SplineComponent.GetTangentAtDistanceAlongSpline` _spline _returnvalue_4 "Local")) (`local.MeshLength`)) true)))